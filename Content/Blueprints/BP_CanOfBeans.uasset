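; BP_CanOfBeans is a holdable, consumable pickup item for BP_ThirdPersonCharacterCustom.
; Overlapping its trigger asks the character to pick it up, and Pickup attaches its root to the hand_r socket.
; Drop detaches it and enables physics and collision on the can.
; PrimaryAction only prints a health gain message without changing health, then clears the character's HeldItem and destroys the actor.
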(event OnComponentBeginOverlap(PickupTrigger)
  (params (OverlappedComponent :type Primitive%20Component%20Object%20Reference) (OtherActor :type Actor%20Object%20Reference) (OtherComp :type Primitive%20Component%20Object%20Reference) (OtherBodyIndex :type Integer) (bFromSweep :type Boolean) (SweepResult :type Hit%20Result%20Structure%20%28by%20ref%29))
  (bind _asbp_third_person_character_custom (Utilities|Casting|CastToBP_ThirdPersonCharacterCustom OtherActor))
  (Default|TrytoPickUp _asbp_third_person_character_custom self))

(event EventBeginPlay)

(event Collision|EventActorBeginOverlap
  (params (OtherActor :type Actor%20Object%20Reference)))

(event EventTick
  (params (DeltaSeconds :type Float%20%28single-precision%29)))

(event EventPickup
  (params (ParentMesh :type Skeletal%20Mesh%20Component%20Object%20Reference))
  (Transformation|AttachComponentToComponent (Variables|Default|GetDefaultSceneRoot) ParentMesh "hand_r" "SnapToTarget" "KeepRelative" "KeepRelative" true))

(event EventDrop
  (Transformation|DetachFromComponent (Variables|Default|GetDefaultSceneRoot) "KeepRelative" "KeepRelative" "KeepRelative" true) ; dont follow hand anymore
  (Physics|SetSimulatePhysics (Variables|Default|GetCan) true) ; use gravity to fall
  (Collision|SetCollisionEnabled (Variables|Default|GetCan) "QueryAndPhysics") ; collide with the ground
)

(event EventPrimaryAction
  (params (ref_ThirdPersonCharCustom :type BP%20Third%20Person%20Character%20Custom%20Object%20Reference))
  (Development|PrintString "+10 Health!")
  (Variables|/Game/Blueprints/BP_ThirdPersonCharacterCustom.BP_ThirdPersonCharacterCustom_C|SetHeldItem ref_ThirdPersonCharCustom 0)
  (Actor|DestroyActor))

(fn ConstructionScript)